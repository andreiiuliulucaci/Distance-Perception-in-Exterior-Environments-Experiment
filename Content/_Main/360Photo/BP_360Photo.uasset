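; BP_360Photo is a Blueprint that displays a 360 photo on a Sphere component and switches which one is shown.
; The Change360PhotoMaterial event switches on an index from 0 to 7, with every case calling SetMaterialByIndex with that same value.
; SetMaterialByIndex applies the matching entry of the MaterialRef array to the sphere's first material slot.
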(event Custom|Change360PhotoMaterial
  (params (NewParam :type Integer))
  (switch int NewParam
    (:0
      (CallFunction|SetMaterialbyIndex NewParam))
    (:1
      (CallFunction|SetMaterialbyIndex NewParam))
    (:2
      (CallFunction|SetMaterialbyIndex NewParam))
    (:3
      (CallFunction|SetMaterialbyIndex NewParam))
    (:4
      (CallFunction|SetMaterialbyIndex NewParam))
    (:5
      (CallFunction|SetMaterialbyIndex NewParam))
    (:6
      (CallFunction|SetMaterialbyIndex NewParam))
    (:7
      (CallFunction|SetMaterialbyIndex NewParam))))

(event EventBeginPlay)

(event Collision|EventActorBeginOverlap
  (params (OtherActor :type Actor%20Object%20Reference)))

(event EventTick
  (params (DeltaSeconds :type Float%20%28single-precision%29)))

(fn ConstructionScript)

(fn SetMaterialbyIndex
  (params (Index :type Integer))
  (Rendering|Material|SetMaterial (Variables|Default|GetSphere) 0 (Utilities|Array|Get(acopy) (Variables|Default|GetMaterialRef) Index)))