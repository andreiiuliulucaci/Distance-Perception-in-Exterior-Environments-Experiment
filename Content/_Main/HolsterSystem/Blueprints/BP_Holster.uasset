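; BP_Holster is a holster actor that holds one item at a time.
; Overlapping the holster mesh captures an "Interactable" actor through a DoOnce, which CanHold? resets after a delay.
; BeginPlay spawns and holsters a configured actor class, and SpawnItemAfterGrab respawns it after a delay if continuous spawning is enabled.
; Holstered items register with their GrabComponent, then snap and attach to the holster.
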(event OnComponentBeginOverlap(HolsterMesh)
  (params (OverlappedComponent :type Primitive%20Component%20Object%20Reference) (OtherActor :type Actor%20Object%20Reference) (OtherComp :type Primitive%20Component%20Object%20Reference) (OtherBodyIndex :type Integer) (bFromSweep :type Boolean) (SweepResult :type Hit%20Result%20Structure%20%28by%20ref%29))
  (Utilities|FlowControl|DoOnce false
    (:Completed
      (if (Actor|ActorHasTag OtherActor "Interactable")
        (if (not (Variables|Default|GetbHasItem?))
          (bind _output_get (Variables|Default|SetHolsteredItem OtherActor))
          (Variables|/Game/VRTemplate/Blueprints/GrabComponent.GrabComponent_C|SetbIsHolstered? (Actor|GetComponentbyClass _output_get "/Game/VRTemplate/Blueprints/GrabComponent.GrabComponent_C") true)
          (Variables|/Game/VRTemplate/Blueprints/GrabComponent.GrabComponent_C|SetHolster (Actor|GetComponentbyClass _output_get "/Game/VRTemplate/Blueprints/GrabComponent.GrabComponent_C") self)
          (Transformation|SetActorLocation (Variables|Default|GetHolsteredItem) (Transformation|GetWorldLocation (Variables|Default|GetHolsterMesh)) false true)
          (Transformation|AttachActorToActor (Variables|Default|GetHolsteredItem) self "Holster" "SnapToTarget" "SnapToTarget" "KeepRelative" true)
          (Variables|Default|SetbHasItem? true))))))

(event Custom|CanHold?
  (Utilities|FlowControl|Delay 1.0)
  (Utilities|FlowControl|DoOnce false) ; enters at Reset
)

(event Custom|SpawnItemAfterGrab
  (if (Variables|Default|GetbContinuallySpawnActor?)
    (Utilities|FlowControl|Delay 1.0)
    (if (not (Variables|Default|GetbHasItem?))
      (bind _returnvalue (Game|SpawnActorfromClass (Variables|Default|GetActorToSpawn) (Math|Transform|MakeTransform "0, 0, 0" "0, 0, 0" (Variables|Default|GetActorSpawnScale)) "Undefined" 0 0))
      (Utilities|IsValid _returnvalue
        (:Is%20Valid
          (if (not (Variables|Default|GetbHasItem?))
            (bind _output_get (Variables|Default|SetHolsteredItem _returnvalue))
            (Variables|/Game/VRTemplate/Blueprints/GrabComponent.GrabComponent_C|SetbIsHolstered? (Actor|GetComponentbyClass _output_get "/Game/VRTemplate/Blueprints/GrabComponent.GrabComponent_C") true)
            (Variables|/Game/VRTemplate/Blueprints/GrabComponent.GrabComponent_C|SetHolster (Actor|GetComponentbyClass _output_get "/Game/VRTemplate/Blueprints/GrabComponent.GrabComponent_C") self)
            (Default|TryGrab (Actor|GetComponentbyClass _output_get "/Game/VRTemplate/Blueprints/GrabComponent.GrabComponent_C"))
            (Transformation|SetActorLocation (Variables|Default|GetHolsteredItem) (Transformation|GetWorldLocation (Variables|Default|GetHolsterMesh)) false true)
            (Transformation|AttachActorToActor (Variables|Default|GetHolsteredItem) self "Holster" "SnapToTarget" "SnapToTarget" "KeepRelative" true)
            (Variables|Default|SetbHasItem? true)))))))

(event EventBeginPlay
  (bind _returnvalue (Game|SpawnActorfromClass (Variables|Default|GetActorToSpawn) (Math|Transform|MakeTransform "0, 0, 0" "0, 0, 0" (Variables|Default|GetActorSpawnScale)) "Undefined" 0 0))
  (Utilities|IsValid _returnvalue
    (:Is%20Valid
      (if (not (Variables|Default|GetbHasItem?))
        (bind _output_get (Variables|Default|SetHolsteredItem _returnvalue))
        (Variables|/Game/VRTemplate/Blueprints/GrabComponent.GrabComponent_C|SetbIsHolstered? (Actor|GetComponentbyClass _output_get "/Game/VRTemplate/Blueprints/GrabComponent.GrabComponent_C") true)
        (Variables|/Game/VRTemplate/Blueprints/GrabComponent.GrabComponent_C|SetHolster (Actor|GetComponentbyClass _output_get "/Game/VRTemplate/Blueprints/GrabComponent.GrabComponent_C") self)
        (Default|TryGrab (Actor|GetComponentbyClass _output_get "/Game/VRTemplate/Blueprints/GrabComponent.GrabComponent_C"))
        (Transformation|SetActorLocation (Variables|Default|GetHolsteredItem) (Transformation|GetWorldLocation (Variables|Default|GetHolsterMesh)) false true)
        (Transformation|AttachActorToActor (Variables|Default|GetHolsteredItem) self "Holster" "SnapToTarget" "SnapToTarget" "KeepRelative" true)
        (Variables|Default|SetbHasItem? true)))))

(fn ConstructionScript)