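; BP_DrawSpline is an actor that draws a path from points stored in the GM_GameInstance.
; BeginPlay appends each stored SplinePoints entry to its Spline in local space.
; Tick adds scaled-down SplineMeshComponents between consecutive points, using spline locations and tangents to shape each segment.
; These components are created anew every frame without removing earlier ones, and the loop index runs up to the array length.
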(event Collision|EventActorBeginOverlap
  (params (OtherActor :type Actor%20Object%20Reference)))

(event EventTick
  (params (DeltaSeconds :type Float%20%28single-precision%29))
  (bind _spline (Variables|Default|GetSpline))
  (bind _spline_2 (Variables|Default|GetSpline))
  (for _index (range 0 (Utilities|Array|Length (Variables|/Game/_Main/Blueprints/DrawingBoundary/GM_GameInstance.GM_GameInstance_C|GetSplinePoints (stale EventBeginPlay _asgm_game_instance))))
    (bind _returnvalue (AddComponent|AddSplineMeshComponent false (Math|Transform|MakeTransform "0, 0, 0" "0, 0, 0" "0.100000,0.100000,0.100000")))
    (SplineMesh|SetForwardAxis _returnvalue "X" true)
    (SplineMesh|SetStartandEnd _returnvalue (Spline|GetLocationatSplinePoint _spline _index "Local") (Spline|GetTangentatSplinePoint _spline _index "Local") (Spline|GetLocationatSplinePoint _spline_2 (+ _index 1) "Local") (Spline|GetTangentatSplinePoint _spline_2 (+ _index 1) "Local") true :!class /Script/Engine.SplineMeshComponent)))

(event EventBeginPlay
  (bind _asgm_game_instance (Utilities|Casting|CastToGM_GameInstance (Game|GetGameInstance)))
  (for _array_element (Variables|/Game/_Main/Blueprints/DrawingBoundary/GM_GameInstance.GM_GameInstance_C|GetSplinePoints _asgm_game_instance)
    (Spline|AddSplinePoint (Variables|Default|GetSpline) _array_element "Local" true)))

(fn ConstructionScript)