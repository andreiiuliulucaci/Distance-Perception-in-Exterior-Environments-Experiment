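; BP_Bilboard is a world-space text billboard actor that turns its text to face the player character.
; The construction script copies the Text variable into the TextRender component, so the label updates in the editor.
; Each tick it smoothly interpolates the text's world rotation toward a look-at rotation aimed at the first player character's location.
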(event EventBeginPlay)

(event Collision|EventActorBeginOverlap
  (params (OtherActor :type Actor%20Object%20Reference)))

(event EventTick
  (params (DeltaSeconds :type Float%20%28single-precision%29))
  (bind _textrender (Variables|Default|GetTextRender))
  (Transformation|SetWorldRotation _textrender (Math|Interpolation|RInterpTo (Transformation|GetWorldRotation _textrender) (Math|Rotator|FindLookatRotation (Transformation|GetWorldLocation (Variables|Default|GetTextRender)) (Transformation|GetActorLocation (Game|GetPlayerCharacter 0))) DeltaSeconds 5.0) false false))

(fn ConstructionScript
  (Rendering|Components|TextRender|SetText (Variables|Default|GetTextRender) (Variables|Default|GetText)))